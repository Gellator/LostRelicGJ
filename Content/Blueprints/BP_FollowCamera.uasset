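; Follow camera actor for a 2D side-scroller that tracks the player and, when set, their current grapple.
; BeginPlay caches the player character; UpdateCamera and ClearCamera set or drop the grapple.
; With a grapple, Tick keeps X and lerps toward the Y midpoint and a Z sum divided by 1.2.
; Otherwise it snaps to the player's X and Z, with Y set to FollowDistance.
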(event `self.ReceiveBeginPlay`
  (bind _as2dside_scroller_character (cast `/Game/Blueprints/2DSideScrollerCharacter` (`GameplayStatics.GetPlayerCharacter` 0))
    (:`then`
      (`self.Setup Camera` _as2dside_scroller_character))
    (:`CastFailed`
      (`KismetSystemLibrary.PrintString` "Failed to find player"))))

(event `self.ReceiveTick`
  (params (DeltaSeconds :type "Float (single-precision)"))
  (bind _returnvalue (`self.K2_GetActorLocation`))
  (bind _player (`self.Player`))
  (bind _current_grapple (`self.Current Grapple`))
  (if (and (`KismetSystemLibrary.IsValid` _player) (`KismetSystemLibrary.IsValid` _current_grapple))
    (`self.K2_SetActorLocation` (`KismetMathLibrary.VLerp` _returnvalue (`KismetMathLibrary.MakeVector` (.x _returnvalue) (/ (+ (.y (`self.K2_GetActorLocation` _player)) (.y (`self.K2_GetActorLocation` _current_grapple))) 2.0) (/ (+ (.z (`self.K2_GetActorLocation` _player)) (.z (`self.K2_GetActorLocation` _current_grapple))) 1.2)) (* (`GameplayStatics.GetWorldDeltaSeconds`) 1.2)))
    (else
      (`self.Follow Player` (`self.Follow Distance`)))))

(fn `Clear Camera`
  (set `self.Current Grapple` null))

(fn `Follow Player`
  (params (`Camera Boom` :type "Float (double-precision)"))
  (bind _player (`self.Player`))
  (bind (_returnvalue_x _returnvalue_y _returnvalue_z) (`KismetMathLibrary.BreakVector` (`self.K2_GetActorLocation` _player)))
  (`/Engine/EditorBlueprintResources/StandardMacros.IsValid` _player
    (:`Is Valid`
      (`self.K2_SetActorLocation` (`KismetMathLibrary.MakeVector` _returnvalue_x `Camera Boom` _returnvalue_z)))))

(fn `Set Player Only Camera`)

(fn `Setup Camera`
  (params (Player :type "/Game/Blueprints/2DSideScrollerCharacter Object Reference"))
  (`/Engine/EditorBlueprintResources/StandardMacros.IsValid` Player
    (:`Is Valid`
      (set `self.Player` Player))))

(fn `Update Camera`
  (params (`New Grapple` :type "/Game/Blueprints/BP_GrapplePoint Object Reference"))
  (`/Engine/EditorBlueprintResources/StandardMacros.IsValid` `New Grapple`
    (:`Is Valid`
      (set `self.Current Grapple` `New Grapple`))))

(fn `UserConstructionScript`)